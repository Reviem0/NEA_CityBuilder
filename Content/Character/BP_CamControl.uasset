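; BP_CamControl is a player-controlled camera rig that pans along its spring arm's axes and turns in steps.
; MoveForward and MoveRight axes feed movement input along the SpringArm's forward and right vectors, so movement follows the current view.
; TurnRight and TurnLeft each play a timeline that lerps the arm's yaw by plus or minus TurnSens, with IsTurning blocking overlapping turns.
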(event EventBeginPlay)

(event Collision|EventActorBeginOverlap
  (params (OtherActor :type Actor%20Object%20Reference)))

(event EventTick
  (params (DeltaSeconds :type Float%20%28single-precision%29)))

(event Input|ActionEvents|InputActionTurnRight
  (params (Key :type Key%20Structure :default "None"))
  (:Pressed
    (if (not (Variables|Default|GetIsTurning?))
      (Variables|Default|SetIsTurning? true)
      (bind _output_get (Variables|Default|SetCurrentArmRotation (Transformation|GetWorldRotation (Variables|Default|GetSpringArm))))
      (bind _newtrack_6 (Timeline|Timeline PlayFromStart)
        (:Update
          (Transformation|SetRelativeRotation (Variables|Default|GetSpringArm) (Math|Rotator|Lerp(Rotator) _output_get (Math|Rotator|MakeRotator (.Roll (Math|Rotator|BreakRotator _output_get)) (.Pitch (Math|Rotator|BreakRotator _output_get)) (+ (.Yaw (Math|Rotator|BreakRotator _output_get)) (Variables|Default|GetTurnSens))) _newtrack_6) false false))
        (:Finished
          (Variables|Default|SetIsTurning? false))))))

(event Input|ActionEvents|InputActionTurnLeft
  (params (Key :type Key%20Structure :default "None"))
  (:Pressed
    (if (not (Variables|Default|GetIsTurning?))
      (Variables|Default|SetIsTurning? true)
      (bind _output_get (Variables|Default|SetCurrentArmRotation (Transformation|GetWorldRotation (Variables|Default|GetSpringArm))))
      (bind _newtrack_6 (Timeline|Timeline_0 PlayFromStart)
        (:Update
          (Transformation|SetRelativeRotation (Variables|Default|GetSpringArm) (Math|Rotator|Lerp(Rotator) _output_get (Math|Rotator|MakeRotator (.Roll (Math|Rotator|BreakRotator _output_get)) (.Pitch (Math|Rotator|BreakRotator _output_get)) (+ (.Yaw (Math|Rotator|BreakRotator _output_get)) (* (Variables|Default|GetTurnSens) -1.0))) _newtrack_6) false false))
        (:Finished
          (Variables|Default|SetIsTurning? false))))))

(event Input|AxisEvents|InputAxisMoveForward
  (params (AxisValue :type Float%20%28single-precision%29))
  (Pawn|Input|AddMovementInput (* (Math|Vector|GetForwardVector (Variables|Default|GetSpringArm)) AxisValue) 1.0 false))

(event Input|AxisEvents|InputAxisMoveRight
  (params (AxisValue :type Float%20%28single-precision%29))
  (Pawn|Input|AddMovementInput (* (Math|Vector|GetRightVector (Variables|Default|GetSpringArm)) AxisValue) 1.0 false))

(fn ConstructionScript)